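; BP_world generates a noise-based terrain mesh once at BeginPlay.
; A FastNoiseWrapper, configured from the Blueprint's noise variables, supplies the height for a scaled XY vertex grid with tiled UVs, printing each sample.
; A running vertex index stitches two triangles per cell, skipping at row ends.
; The arrays feed one ProceduralMesh section with no supplied normals, which then receives the Material.
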(event EventBeginPlay
  (bind _returnvalue (Game|ConstructObjectfromClass "/Script/FastNoiseGenerator.FastNoiseWrapper"))
  (bind _output_get (Variables|Default|SetNoise _returnvalue))
  (Class|FastNoiseWrapper|SetupFastNoise _output_get (Variables|Default|GetNoise%20Type_0) (Variables|Default|GetSeed) (Variables|Default|GetFrequency) (Variables|Default|GetInterp) (Variables|Default|GetFractaltype) (Variables|Default|GetOctaves) (Variables|Default|GetLacunarity) (Variables|Default|GetGain) (Variables|Default|GetCellular%20Jitter) (Variables|Default|GetCellular%20Distance%20Function) (Variables|Default|GetCellular%20Return%20Type))
  (CallFunction|CreateVertices)
  (CallFunction|CreateTriangles)
  (Class|ProceduralMeshComponent|CreateMeshSectionLinearColor (Variables|Default|GetProceduralMesh) 0 (Variables|Default|GetVertices) (Variables|Default|GetTriangles) 0 (Variables|Default|GetUV0) 0 0 0 0 0 false false)
  (Rendering|Material|SetMaterial (Variables|Default|GetProceduralMesh) 0 (Variables|Default|GetMaterial)))

(fn ConstructionScript)

(fn CreateVertices
  (for _index (range 0 (Variables|Default|GetXSize))
    (LocalVariables|SetX _index)
    (for _index_2 (range 0 (Variables|Default|GetYSize))
      (LocalVariables|SetY _index_2)
      (Utilities|Array|Add (Variables|Default|GetVertices) (Math|Vector|MakeVector (* (LocalVariables|GetX) (Variables|Default|GetScale)) (* (LocalVariables|GetY) (Variables|Default|GetScale)) (* (Variables|Default|GetZMultiplier) (Class|FastNoiseWrapper|GetNoise2D (Variables|Default|GetNoise) (+ (Math|Conversions|ToFloat(Integer) (LocalVariables|GetX)) 0.1) (+ (Math|Conversions|ToFloat(Integer) (LocalVariables|GetY)) 0.1)))))
      (Development|PrintString (Utilities|String|ToString(Float) (Class|FastNoiseWrapper|GetNoise2D (Variables|Default|GetNoise) (+ (Math|Conversions|ToFloat(Integer) (LocalVariables|GetX)) 0.1) (+ (Math|Conversions|ToFloat(Integer) (LocalVariables|GetY)) 0.1))))
      (Utilities|Array|Add (Variables|Default|GetUV0) (Math|Vector2D|MakeVector2D (* (LocalVariables|GetX) (Variables|Default|GetUVScale)) (* (LocalVariables|GetY) (Variables|Default|GetUVScale)))))))

(fn CreateTriangles
  (for _index (range 0 (- (Variables|Default|GetXSize) 1))
    (for _index_2 (range 0 (- (Variables|Default|GetYSize) 1))
      (Utilities|Array|Add (Variables|Default|GetTriangles) (LocalVariables|GetVertex))
      (Utilities|Array|Add (Variables|Default|GetTriangles) (+ (LocalVariables|GetVertex) 1))
      (Utilities|Array|Add (Variables|Default|GetTriangles) (+ (Variables|Default|GetYSize) (LocalVariables|GetVertex) 1))
      (Utilities|Array|Add (Variables|Default|GetTriangles) (+ (LocalVariables|GetVertex) 1))
      (Utilities|Array|Add (Variables|Default|GetTriangles) (+ (Variables|Default|GetYSize) 2 (LocalVariables|GetVertex)))
      (Utilities|Array|Add (Variables|Default|GetTriangles) (+ (Variables|Default|GetYSize) (LocalVariables|GetVertex) 1))
      (Math|Integer|IncrementInt (LocalVariables|GetVertex)))
    (Math|Integer|IncrementInt (LocalVariables|GetVertex))))