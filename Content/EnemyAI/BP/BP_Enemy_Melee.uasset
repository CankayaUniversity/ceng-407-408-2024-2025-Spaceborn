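; Melee enemy Blueprint that overrides its parent's setup with a montage-driven attack.
; Attack plays the montage and makes the damage system uninterruptible until it completes or is interrupted, then calls OnAttackEnd.
; On montage notify, a forward sphere trace against Pawns, long for melee and with debug drawing on, sends damage info to the hit actor through a TakeDamage message.
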(event EventBeginPlay
  (|CallParentFunction))

(event EventAttack
  (bind _returnvalue (Transformation|GetActorLocation))
  (bind _notifyname (Animation|Montage|PlayMontage (Variables|Character|GetMesh) "/Game/Characters/Mannequins/Animations/Manny/yalandan_attack.yalandan_attack")
    (:then
      (Variables|/Game/EnemyAI/DamageSystem/BPC_DamageSystem.BPC_DamageSystem_C|SetIsInterruptible (Variables|Default|GetBPC_DamageSystem) false))
    (:OnCompleted
      (Default|CallOnAttackEnd :!label _label)
      (Variables|/Game/EnemyAI/DamageSystem/BPC_DamageSystem.BPC_DamageSystem_C|SetIsInterruptible (Variables|Default|GetBPC_DamageSystem) true))
    (:OnInterrupted
      (goto _label))
    (:OnNotifyBegin
      (switch name _notifyname
        (:Slash
          (bind (_outhit _returnvalue_2) (Collision|SphereTraceForObjects _returnvalue (+ _returnvalue (* (Transformation|GetActorForwardVector) 2e+03)) 2e+01 (Utilities|Array|MakeArray "ObjectTypeQuery3") false 0 "ForDuration"))
          (if _returnvalue_2
            (Class|BPIDamagable|TakeDamage(Message) (.HitActor (Collision|BreakHitResult _outhit)) (Utilities|Struct|MakeS_DamageInfo 2e+01 "NewEnumerator3"))))))))

(fn ConstructionScript
  (|CallParentFunction))