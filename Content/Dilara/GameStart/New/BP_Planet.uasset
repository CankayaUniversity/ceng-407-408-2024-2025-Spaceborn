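; BP_Planet is a planet actor with an info widget and a SpringArm that can be orbited.
; BeginPlay copies its Name and Info into the Info_UI widget.
; Tick polls BP_FirstPersonCharacter; while ChangedCamera is set, it shows the cursor and adds a new Back_UI every frame.
; Held left or right mouse flags yaw the SpringArm by a fixed per-frame step, zeroing pitch and roll.
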(event EventBeginPlay
  (bind _asinfo_ui (Utilities|Casting|CastToInfo_UI (UserInterface|GetWidget (Variables|Default|GetWidget))))
  (Variables|/Game/Dilara/GameStart/New/Info_UI.Info_UI_C|SetName _asinfo_ui (Variables|Default|Getname))
  (Variables|/Game/Dilara/GameStart/New/Info_UI.Info_UI_C|SetInfo _asinfo_ui (Variables|Default|Getinfo)))

(event EventTick
  (params (DeltaSeconds :type Float%20%28single-precision%29))
  (bind _springarm (Variables|Default|GetSpringArm))
  (bind _springarm_2 (Variables|Default|GetSpringArm))
  (bind _returnvalue (Actor|GetActorOfClass "/Game/FirstPerson/Blueprints/BP_FirstPersonCharacter.BP_FirstPersonCharacter_C"))
  (if (Variables|/Game/FirstPerson/Blueprints/BP_FirstPersonCharacter.BP_FirstPersonCharacter_C|GetChangedCamera _returnvalue)
    (Variables|/Script/Engine.PlayerController|SetbShowMouseCursor (Game|GetPlayerController 0) true)
    (bind _returnvalue_2 (UserInterface|CreateWidget "/Game/Dilara/GameStart/New/Back_UI.Back_UI_C"))
    (UserInterface|Viewport|AddtoViewport _returnvalue_2 0)
    (if (Variables|/Game/FirstPerson/Blueprints/BP_FirstPersonCharacter.BP_FirstPersonCharacter_C|GetPressedLeftMouseButton _returnvalue)
      (Transformation|SetWorldRotation _springarm (Math|Rotator|MakeRotator 0.0 0.0 (+ (.yaw (Transformation|GetWorldRotation _springarm)) 2.0)) false false))
    (if (Variables|/Game/FirstPerson/Blueprints/BP_FirstPersonCharacter.BP_FirstPersonCharacter_C|GetPressedRightMouseButton _returnvalue)
      (Transformation|SetWorldRotation _springarm_2 (Math|Rotator|MakeRotator 0.0 0.0 (- (.yaw (Transformation|GetWorldRotation _springarm_2)) 2.0)) false false))))

(fn ConstructionScript)